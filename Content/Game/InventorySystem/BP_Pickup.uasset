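; BP_Pickup is a world item the player can look at and pick up into their inventory.
; A data asset supplies the mesh, set in the construction script, and the name shown with a "Pick up" prompt on look-at.
; Interacting adds the item and quantity to the player's InventorySystem, then destroys the actor if the add succeeds and the asset marks it destroyed on pickup.
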(event `/Game/BPI_Interact.InteractWith`
  (params (PlayerCharacter :type "/Game/FirstPerson/Blueprints/BP_FirstPersonCharacter Object Reference"))
  (bind _dataasset (`self.DataAsset`))
  (bind _success (`/Game/Game/InventorySystem/InventorySystem.AddToInventory` (`/Game/FirstPerson/Blueprints/BP_FirstPersonCharacter.InventorySystem` PlayerCharacter) _dataasset (`self.Quantity`)))
  (if (and _success (`/Game/Game/InventorySystem/Data/DA_Item.IsDestroyedOnPickup` _dataasset))
    (`self.K2_DestroyActor`)))

(fn `LookAt`
  (returns (Verb :type Text) (Noun :type Text))
  (return "Pick up" (`/Game/Game/InventorySystem/Data/DA_Item.Name` (`self.DataAsset`))))

(fn `UserConstructionScript`
  (bind _dataasset (`self.DataAsset`)
    (:`then`
      (`StaticMeshComponent.SetStaticMesh` (`self.StaticMesh`) (`/Game/Game/InventorySystem/Data/DA_Item.StaticMesh` _dataasset)))
    (:`else`)))