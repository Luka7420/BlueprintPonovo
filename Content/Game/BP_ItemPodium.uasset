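; BP_ItemPodium is an interactable podium that takes a required item from the player and fires a trigger.
; Interactwith checks the interacting character's InventorySystem for one of the Item, removes it, displays the item's static mesh on the podium, then calls OnTriggered with true.
; LookAt checks player 0's inventory to return a "Place" or "Requires" prompt with the item's name.
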(event `/Game/BPI_Interact.InteractWith`
  (params (PlayerCharacter :type "/Game/FirstPerson/Blueprints/BP_FirstPersonCharacter Object Reference"))
  (bind _inventorysystem (`/Game/FirstPerson/Blueprints/BP_FirstPersonCharacter.InventorySystem` PlayerCharacter))
  (bind _item (`self.Item`))
  (bind _return (`/Game/Game/InventorySystem/InventorySystem.QueryInventory` _inventorysystem (`self.Item`) 1))
  (if _return
    (`/Game/Game/InventorySystem/InventorySystem.RemoveFromInventory` _inventorysystem _item 1)
    (`StaticMeshComponent.SetStaticMesh` (`self.StaticMesh`) (`/Game/Game/InventorySystem/Data/DA_Item.StaticMesh` _item))
    (`self.OnTriggered` true)))

(fn `LookAt`
  (returns (Verb :type Text) (Noun :type Text))
  (bind _name (`/Game/Game/InventorySystem/Data/DA_Item.Name` (`self.Item`)))
  (bind _return (`/Game/Game/InventorySystem/InventorySystem.QueryInventory` (`self.GetComponentByClass` (`GameplayStatics.GetPlayerCharacter` 0) "/Game/Game/InventorySystem/InventorySystem.InventorySystem_C") (`self.Item`) 1))
  (if _return
    (return "Place" _name)
    (else
      (return "Requires" _name))))

(fn `UserConstructionScript`
  (`parent.UserConstructionScript`))