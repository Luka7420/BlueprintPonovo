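; Lockable elevator that the player calls by interacting, shown with a "Call Elevator" look-at verb and noun.
; When unlocked, interaction plays a timeline that raises the Cube; the player leaving the overlap reverses it.
; A Trigger's state locks or unlocks the elevator, and a point light shows red for locked or green for unlocked.
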(event `self.ReceiveActorBeginOverlap`
  (params (OtherActor :type "Actor Object Reference")))

(event `self.ReceiveActorEndOverlap`
  (params (OtherActor :type "Actor Object Reference"))
  (if (== OtherActor (`GameplayStatics.GetPlayerCharacter` 0))
    (`self.CloseElevator`)))

(event `OpenElevator`
  (if (not (`self.IsLocked`))
    (bind (_direction _position) (`Timeline|ElevatorTime` :!label _label)
      (:`Update`
        (`SceneComponent.K2_SetRelativeLocation` (`self.Cube`) (* (0.0 0.0 220.0) _position) false false)))))

(event `CloseElevator`
  (goto _label :!via `Reverse`))

(event `self.Trigger.OnTriggered`
  (params (IsTriggered :type Boolean))
  (if IsTriggered
    (`self.UnlockElevator`)
    (else
      (`self.LockElevator`))))

(event `/Game/BPI_Interact.InteractWith`
  (params (PlayerCharacter :type "/Game/FirstPerson/Blueprints/BP_FirstPersonCharacter Object Reference"))
  (`self.OpenElevator`))

(fn `LockElevator`
  (bind _output_get (set `self.IsLocked` true))
  (`LightComponent.SetLightColor` (`self.PointLight`) (`KismetMathLibrary.SelectColor` (struct :`R` 1.0 :`G` 0.012087 :`A` 1.0) (struct :`G` 1.0 :`B` 0.30166 :`A` 1.0) _output_get) true))

(fn `LookAt`
  (returns (Verb :type Text) (Noun :type Text))
  (return "Call" "Elevator"))

(fn `UnlockElevator`
  (bind _output_get (set `self.IsLocked` false))
  (`LightComponent.SetLightColor` (`self.PointLight`) (`KismetMathLibrary.SelectColor` (struct :`R` 1.0 :`G` 0.012087 :`A` 1.0) (struct :`G` 1.0 :`B` 0.30166 :`A` 1.0) _output_get) true))

(fn `UserConstructionScript`
  (`LightComponent.SetLightColor` (`self.PointLight`) (`KismetMathLibrary.SelectColor` (struct :`R` 1.0 :`G` 0.012087 :`A` 1.0) (struct :`G` 1.0 :`B` 0.30166 :`A` 1.0) (`self.IsLocked`)) true))